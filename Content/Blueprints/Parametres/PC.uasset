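; Player controller that acts as the UI hub, showing the main menu, pause, tutorial, controls, options, end-of-game screen and player HUD.
; Each display event lazily creates its widget, caches it and adds it to the viewport; the end screen also pauses the game.
; The Pause input clears all widgets and opens the pause menu only when the game mode's NouvellePartie flag is set.
; Showing the HUD also inserts a new mission widget into its slot after a short delay.
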(event `self.ReceiveBeginPlay`
  (bind _asgm (cast `/Game/Blueprints/Parametres/GM` (`GameplayStatics.GetGameMode`)))
  (set `self.ModeDeJeu` _asgm)
  (bind _aspersonnage (cast `/Game/Blueprints/Personnage` (`GameplayStatics.GetPlayerCharacter` 0)))
  (set `self.Personnage` _aspersonnage))

(event `InputAction|Pause`
  (params (Key :type "Key Structure"))
  (:`Pressed`
    (if (`/Game/Blueprints/Parametres/GM.NouvellePartie` (`self.ModeDeJeu`))
      (`WidgetLayoutLibrary.RemoveAllWidgets`)
      (`self.AfficherPause`))))

(event `AfficherPause`
  (`/Engine/EditorBlueprintResources/StandardMacros.IsValid` (`self.w_MenuPause`)
    (:`Is Valid`
      _)
    (:`Is Not Valid`
      (bind _returnvalue (`|CreateWidget` "/Game/Blueprints/Widgets/Menu/Pause.Pause_C"))
      (bind _output_get (set `self.w_MenuPause` _returnvalue))))
  (`UserWidget.AddToViewport` _output_get 0))

(event `AfficherTutoriel`
  (`/Engine/EditorBlueprintResources/StandardMacros.IsValid` (`self.w_MenuTutoriel`)
    (:`Is Valid`
      _)
    (:`Is Not Valid`
      (bind _returnvalue (`|CreateWidget` "/Game/Blueprints/Widgets/Menu/Tutoriel.Tutoriel_C"))
      (bind _output_get (set `self.w_MenuTutoriel` _returnvalue))))
  (`UserWidget.AddToViewport` _output_get 0))

(event `AfficherMenu`
  (`/Engine/EditorBlueprintResources/StandardMacros.IsValid` (`self.w_MenuPrincipal`)
    (:`Is Valid`
      _)
    (:`Is Not Valid`
      (bind _returnvalue (`|CreateWidget` "/Game/Blueprints/Widgets/Menu/Menu.Menu_C"))
      (bind _output_get (set `self.w_MenuPrincipal` _returnvalue))))
  (`UserWidget.AddToViewport` _output_get 0))

(event `AfficherInterfaceUtilisateurDuPerso`
  (`/Engine/EditorBlueprintResources/StandardMacros.IsValid` (`self.w_InterfaceUtilisateur`)
    (:`Is Valid`
      _)
    (:`Is Not Valid`
      (bind _returnvalue (`|CreateWidget` "/Game/Blueprints/Widgets/IU/InterfaceDuJoueur.InterfaceDuJoueur_C"))
      (bind _output_get (set `self.w_InterfaceUtilisateur` _returnvalue))))
  (`UserWidget.AddToViewport` _output_get 0)
  (`self.AfficherTexteMission`))

(event `AfficherMenuControl`
  (`/Engine/EditorBlueprintResources/StandardMacros.IsValid` (`self.w_MenuControl`)
    (:`Is Valid`
      _)
    (:`Is Not Valid`
      (bind _returnvalue (`|CreateWidget` "/Game/Blueprints/Widgets/Menu/Control.Control_C"))
      (bind _output_get (set `self.w_MenuControl` _returnvalue))))
  (`UserWidget.AddToViewport` _output_get 0))

(event `AfficherFinDuJEu`
  (`GameplayStatics.SetGamePaused` true)
  (`/Engine/EditorBlueprintResources/StandardMacros.IsValid` (`self.w_MenuFinDuJeu`)
    (:`Is Valid`
      _)
    (:`Is Not Valid`
      (bind _returnvalue (`|CreateWidget` "/Game/Blueprints/Widgets/Menu/FinDePartie.FinDePartie_C" null self))
      (bind _output_get (set `self.w_MenuFinDuJeu` _returnvalue))))
  (`UserWidget.AddToViewport` _output_get 0))

(event `AfficherTexteMission`
  (`KismetSystemLibrary.Delay` 2.0)
  (bind _returnvalue (`|CreateWidget` "/Game/Blueprints/Widgets/IU/Mission.Mission_C"))
  (`PanelWidget.AddChild` (`/Game/Blueprints/Widgets/IU/InterfaceDuJoueur.Emplacement_Widget_Mission` (`self.w_InterfaceUtilisateur`)) _returnvalue))

(event `MenuOptions`
  (`/Engine/EditorBlueprintResources/StandardMacros.IsValid` (`self.w_MenuOptions`)
    (:`Is Valid`
      _)
    (:`Is Not Valid`
      (bind _returnvalue (`|CreateWidget` "/Game/Blueprints/Widgets/Menu/Options.Options_C"))
      (bind _output_get (set `self.w_MenuOptions` _returnvalue))))
  (`UserWidget.AddToViewport` _output_get 0))

(fn `UserConstructionScript`)