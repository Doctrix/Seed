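; Player controller that manages the game's UI screens: pause, tutorial, main menu, HUD, controls and end-of-game.
; Each show event lazily creates its widget, caches the reference and adds it to the viewport; the end-of-game event also pauses the game.
; The Pause input clears all widgets and shows the pause screen, only when the GM game mode's NouvellePartie flag is set.
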(event `self.ReceiveBeginPlay`
  (bind _asgm (cast `/Game/Blueprints/GM` (`GameplayStatics.GetGameMode`)))
  (set `self.GameMode_REF` _asgm))

(event `InputAction|Pause`
  (params (Key :type "Key Structure"))
  (:`Pressed`
    (if (`/Game/Blueprints/GM.NouvellePartie` (`self.GameMode_REF`))
      (`WidgetLayoutLibrary.RemoveAllWidgets`)
      (`self.AfficherPause`))))

(event `AfficherPause`
  (`/Engine/EditorBlueprintResources/StandardMacros.IsValid` (`self.Pause_Widget_REF`)
    (:`Is Valid`
      _)
    (:`Is Not Valid`
      (bind _returnvalue (`|CreateWidget` "/Game/Blueprints/Widgets/Pause.Pause_C"))
      (bind _output_get (set `self.Pause_Widget_REF` _returnvalue))))
  (`UserWidget.AddToViewport` _output_get 0))

(event `AfficherTutoriel`
  (`/Engine/EditorBlueprintResources/StandardMacros.IsValid` (`self.Tutoriel_Widget_REF`)
    (:`Is Valid`
      _)
    (:`Is Not Valid`
      (bind _returnvalue (`|CreateWidget` "/Game/Blueprints/Widgets/Tutoriel.Tutoriel_C"))
      (bind _output_get (set `self.Tutoriel_Widget_REF` _returnvalue))))
  (`UserWidget.AddToViewport` _output_get 0))

(event `AfficherMenu`
  (`/Engine/EditorBlueprintResources/StandardMacros.IsValid` (`self.MenuWidget_Widget_REF`)
    (:`Is Valid`
      _)
    (:`Is Not Valid`
      (bind _returnvalue (`|CreateWidget` "/Game/Blueprints/Widgets/Menu.Menu_C"))
      (bind _output_get (set `self.MenuWidget_Widget_REF` _returnvalue))))
  (`UserWidget.AddToViewport` _output_get 0))

(event `AfficherInterfaceUtilisateurDuPerso`
  (`/Engine/EditorBlueprintResources/StandardMacros.IsValid` (`self.InterfaceUtilisateur_Widget_REF`)
    (:`Is Valid`
      _)
    (:`Is Not Valid`
      (bind _returnvalue (`|CreateWidget` "/Game/Blueprints/Widgets/IU.IU_C"))
      (bind _output_get (set `self.InterfaceUtilisateur_Widget_REF` _returnvalue))))
  (`UserWidget.AddToViewport` _output_get 0))

(event `AfficherMenuControl`
  (`/Engine/EditorBlueprintResources/StandardMacros.IsValid` (`self.Control_Widget_REF`)
    (:`Is Valid`
      _)
    (:`Is Not Valid`
      (bind _returnvalue (`|CreateWidget` "/Game/Blueprints/Widgets/Control.Control_C"))
      (bind _output_get (set `self.Control_Widget_REF` _returnvalue))))
  (`UserWidget.AddToViewport` _output_get 0))

(event `AfficherFinDuJEu`
  (`GameplayStatics.SetGamePaused` true)
  (`/Engine/EditorBlueprintResources/StandardMacros.IsValid` (`self.FinDuJeu_Widget_REF`)
    (:`Is Valid`
      _)
    (:`Is Not Valid`
      (bind _returnvalue (`|CreateWidget` "/Game/Blueprints/Widgets/FinDePartie.FinDePartie_C" null self))
      (bind _output_get (set `self.FinDuJeu_Widget_REF` _returnvalue))))
  (`UserWidget.AddToViewport` _output_get 0))

(fn `UserConstructionScript`)