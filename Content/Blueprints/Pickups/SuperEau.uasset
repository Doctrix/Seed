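; SuperEau is a super-water pickup that the player (Personnage) or an Ennemi collects by overlapping its sphere.
; Either collector flags it collected and lowers the GM game mode's on-ground count, with Tick destroying the flagged actor.
; Only the player gains the water quantity and super-water gauge progress, set to a fixed value when already at maximum.
; The construction script sizes the collision sphere from a radius variable.
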(event `self.ReceiveTick`
  (params (DeltaSeconds :type "Float (single-precision)"))
  (if (`self.Recolter?`)
    (`self.K2_DestroyActor`))
  (set `self.Recolter?` false))

(event `self.Sphere.OnComponentBeginOverlap`
  (params (OverlappedComponent :type "PrimitiveComponent Object Reference") (OtherActor :type "Actor Object Reference") (OtherComp :type "PrimitiveComponent Object Reference") (OtherBodyIndex :type Integer) (bFromSweep :type Boolean) (SweepResult :type "HitResult Structure (by ref)"))
  (`|ExecutionSequence`
    (:`then_0`
      (bind _aspersonnage (cast `/Game/Blueprints/Personnage` OtherActor))
      (set `self.Recolter?` true)
      (set `self.Hero?` true))
    (:`then_1`
      (cast `/Game/Blueprints/IA/Ennemi` OtherActor)
      (set `self.Recolter?` true)
      (set `self.Hero?` false)))
  (bind _asgm (cast `/Game/Blueprints/Parametres/GM` (`GameplayStatics.GetGameMode`)))
  (set `/Game/Blueprints/Parametres/GM.MontantSuperEauAuSol` (- (`/Game/Blueprints/Parametres/GM.MontantSuperEauAuSol` _asgm) 1) _asgm)
  (if (`self.Hero?`)
    (set `/Game/Blueprints/Personnage.QuantiteEauRecolter` (+ (`self.Quantite`) (`/Game/Blueprints/Personnage.QuantiteEauRecolter` _aspersonnage)) _aspersonnage)
    (bind _supereaurecolter (`/Game/Blueprints/Personnage.SuperEauRecolter` _aspersonnage))
    (if (== _supereaurecolter (`/Game/Blueprints/Personnage.SuperEauMaxRecolter` _aspersonnage))
      (set `/Game/Blueprints/Personnage.SuperEauRecolter` 100.0 _aspersonnage)
      (else
        (set `/Game/Blueprints/Personnage.SuperEauRecolter` (+ _supereaurecolter 4.0) _aspersonnage)))))

(fn `UserConstructionScript`
  (`SphereComponent.SetSphereRadius` (`self.Sphere`) (`self.RayonDeLaSphereCollision`) false))