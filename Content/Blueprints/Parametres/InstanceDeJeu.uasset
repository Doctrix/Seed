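; Game instance that connects the game to the GameJolt service and awards trophies to the player.
; On Init it creates a GameJolt API object and initializes it with the game's key and ID.
; AchieveTrophy maps a selection (first connection or Canon AO) to a trophy ID, stores the reward result in an unlocked flag, then clears that flag after a short delay.
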(event `self.ReceiveInit`
  (bind _output_get (set `self.GameJoltAPI` (`UEGameJoltAPI.Create`)))
  (`UEGameJoltAPI.Init` _output_get (`self.Key`) (`self.GameID`)))

(event `AchieveTrophy`
  (params (Selection :type "/Game/Blueprints/Trophee_Enum Enum" :default "NewEnumerator0"))
  (bind _gamejoltapi (`self.GameJoltAPI`))
  (switch `/Game/Blueprints/Trophee_Enum` Selection
    (:`NewEnumerator0`
      (bind _returnvalue (`UEGameJoltAPI.RewardTrophy` _gamejoltapi 120449))
      (set `self.TropheDebloquer` _returnvalue))
    (:`NewEnumerator1`
      (bind _returnvalue_2 (`UEGameJoltAPI.RewardTrophy` _gamejoltapi 120625))
      (set `self.TropheDebloquer` _returnvalue_2)))
  (`KismetSystemLibrary.Delay` 3.0)
  (set `self.TropheDebloquer` false))