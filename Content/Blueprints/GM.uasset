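; Game manager Blueprint (GM) that runs the in-game clock, day/night HUD and end screen.
; While NouvellePartie is set, Tick calls Temps, which advances time, updates the sky sphere's sun and switches the HUD's sun/moon icon.
; Midnight sets NouvelleJournee, which triggers a thirst-multiplier notification, and the first day change calls Evolution on the Graine (seed) actor.
; When Graine's FinDuJEu is true, EcranDeFin shows FinDePartie and disables character input.
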(event `self.ReceiveBeginPlay`
  (bind _returnvalue (`GameplayStatics.GetActorOfClass` "/Engine/EngineSky/BP_Sky_Sphere.BP_Sky_Sphere_C"))
  (set `self.Ciel` _returnvalue))

(event `self.ReceiveTick`
  (params (DeltaSeconds :type "Float (single-precision)"))
  (bind _iu_ref (`self.IU_REF`))
  (`|ExecutionSequence`
    (:`then_0`
      (if (`self.NouvellePartie`)
        (`self.Temps`)
        (if (`self.NouvelleJournee`)
          (`/Game/Blueprints/IU.AfficherNotifMultiplicateurDeSoif` _iu_ref true)
          (`KismetSystemLibrary.Delay` 3.0)
          (`/Game/Blueprints/IU.AfficherNotifMultiplicateurDeSoif` _iu_ref false))))
    (:`then_1`
      (bind _returnvalue (`GameplayStatics.GetActorOfClass` "/Game/Blueprints/Graine.Graine_C"))
      (if (`/Game/Blueprints/Graine.FinDuJEu` _returnvalue)
        (`self.EcranDeFin`)))))

(event `Temps`
  (bind _iu_ref (`self.IU_REF`))
  (bind _heure (`self.heure`))
  (bind _minutes (`self.minutes`))
  (bind _heure_2 (`self.heure`))
  (bind _image_temps (`/Game/Blueprints/IU.Image_temps` _iu_ref))
  (bind _border_temps (`/Game/Blueprints/IU.Border_temps` _iu_ref))
  (`KismetSystemLibrary.Delay` 0.01)
  (set `self.secondes` (+ (* (`self.secondes`) 4.0) 1.0))
  (if (> (`self.secondes`) 59.0)
    (set `self.secondes` 0.0)
    (set `self.minutes` (+ _minutes 1.0))
    (if (> _minutes 59.0)
      (set `self.minutes` 0.0)
      (set `self.heure` (+ _heure_2 1.0))
      (if (> _heure_2 23.0)
        (set `self.heure` 0.0)
        (set `self.NouvelleJournee` true)
        (bind _output_get (set `self.jour` (+ (`self.jour`) 1.0)))
        (if (== _output_get 1.0)
          (bind _returnvalue (`GameplayStatics.GetActorOfClass` "/Game/Blueprints/Graine.Graine_C"))
          (`/Game/Blueprints/Graine.evolution` _returnvalue)))))
  (`/Game/Blueprints/IU.ObtenirLeTemps` _iu_ref _heure (`self.minutes`) (`self.secondes`) (`self.jour`))
  (`/Engine/EngineSky/BP_Sky_Sphere.UpdateSunDirection` (`self.Ciel`))
  (if (>= _heure 19.0)
    (`Image.SetBrushFromTexture` _image_temps "/Game/Textures/lune_seed.lune_seed" true :!label _label)
    (`Border.SetBrushColor` _border_temps (struct :`R` 0.015625 :`G` 0.001799 :`A` 0.8))
    (elif (<= _heure 6.0)
      (goto _label)
      (else
        (`Image.SetBrushFromTexture` _image_temps "/Game/Textures/soleil_seed.soleil_seed" true)
        (`Border.SetBrushColor` _border_temps (struct :`R` 0.64448 :`G` 0.074214 :`A` 0.8))))))

(event `AfficherIUDuPerso`
  (`/Engine/EditorBlueprintResources/StandardMacros.IsValid` (`self.IU_REF`)
    (:`Is Valid`
      _)
    (:`Is Not Valid`
      (bind _returnvalue (`|CreateWidget` "/Game/Blueprints/IU.IU_C"))
      (bind _output_get (set `self.IU_REF` _returnvalue))))
  (`UserWidget.AddToViewport` _output_get 0))

(fn `EcranDeFin`
  (bind _returnvalue (`GameplayStatics.GetPlayerController` 0))
  (`WidgetLayoutLibrary.RemoveAllWidgets`)
  (bind _returnvalue_2 (`|CreateWidget` "/Game/Blueprints/FinDePartie.FinDePartie_C"))
  (`UserWidget.AddToViewport` _returnvalue_2 0)
  (`self.DisableInput` (`GameplayStatics.GetPlayerCharacter` 0) _returnvalue)
  (set `PlayerController.bShowMouseCursor` true _returnvalue)
  (`WidgetBlueprintLibrary.SetInputMode_GameOnly` _returnvalue))

(fn `UserConstructionScript`)