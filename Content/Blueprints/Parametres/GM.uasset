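; GM, apparently the game mode, runs the game clock and day/night cycle, plus menu music and looping menu sequence.
; CastsRef caches controller, character, sky and Graine (seed) references on BeginPlay.
; During a new game, Tick calls Temps, whose Delay paces the clock feeding the HUD, sun and sun/moon icon.
; Day rollover triggers seed evolution on day 1; Tick handles the thirst-multiplier notification and end-of-game screen.
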(event `MusiqueMenu`
  ;[1 1 1] Son du jeu
  (bind _returnvalue (`GameplayStatics.CreateSound2D` (`self.Musique`) 1.0 1.0 0.0 null))
  (bind _output_get (set `self.Audio` _returnvalue))
  (`AudioComponent.Play` _output_get 0.0))

(event `self.ReceiveBeginPlay`
  (`self.CastsRef`))

(event `Temps`
  (bind _heure (`self.heure`))
  (bind _minutes (`self.minutes`))
  (bind _heure_2 (`self.heure`))
  (bind _w_interfaceutilisateur (`/Game/Blueprints/Parametres/PC.w_InterfaceUtilisateur` (`self.ControlleurDuJoueur_REF`)))
  (bind _avatar_jour_nuit (`/Game/Blueprints/Widgets/InterfaceDuJoueur.Avatar_Jour_Nuit` _w_interfaceutilisateur))
  (bind _bordure_avatar_jour_nuit (`/Game/Blueprints/Widgets/InterfaceDuJoueur.Bordure_Avatar_Jour_Nuit` _w_interfaceutilisateur))
  (`KismetSystemLibrary.Delay` (/ (`self.VitesseDuTemps`) 10.0))
  (set `self.secondes` (+ (`self.secondes`) 1.0))
  (if (> (`self.secondes`) 59.0)
    (set `self.secondes` 0.0)
    (set `self.minutes` (+ _minutes 1.0))
    (if (> _minutes 59.0)
      (set `self.minutes` 0.0)
      (set `self.heure` (+ _heure_2 1.0))
      (if (> _heure_2 23.0)
        (set `self.heure` 0.0)
        (set `self.NouvelleJourner` true)
        (bind _output_get (set `self.jour` (+ (`self.jour`) 1.0)))
        (if (== _output_get 1.0)
          (`/Game/Blueprints/Graine.Evolution` (`self.Graine_REF`))))))
  (`/Game/Blueprints/Widgets/InterfaceDuJoueur.LeTempsEnCours` _w_interfaceutilisateur _heure (`self.minutes`) (`self.secondes`) (`self.jour`))
  (`/Engine/EngineSky/BP_Sky_Sphere.UpdateSunDirection` (`self.Ciel_REF`))
  (if (>= _heure 19.0)
    (`Image.SetBrushFromTexture` _avatar_jour_nuit "/Game/Textures/lune_seed.lune_seed" true :!label _label)
    (`Border.SetBrushColor` _bordure_avatar_jour_nuit (struct :`R` 0.015625 :`G` 0.001799 :`A` 0.8))
    (elif (<= _heure 6.0)
      (goto _label)
      (else
        (`Image.SetBrushFromTexture` _avatar_jour_nuit "/Game/Textures/soleil_seed.soleil_seed" true)
        (`Border.SetBrushColor` _bordure_avatar_jour_nuit (struct :`R` 0.64448 :`G` 0.074214 :`A` 0.8))))))

(event `self.ReceiveTick`
  (params (DeltaSeconds :type "Float (single-precision)"))
  (bind _w_interfaceutilisateur (`/Game/Blueprints/Parametres/PC.w_InterfaceUtilisateur` (`self.ControlleurDuJoueur_REF`)))
  (`|ExecutionSequence`
    (:`then_0`
      (if (`self.NouvellePartie`)
        (`self.Temps`)
        (if (`self.NouvelleJourner`)
          (`/Game/Blueprints/Widgets/InterfaceDuJoueur.NotificationMultiplicateurDeSoif` _w_interfaceutilisateur true)
          (`KismetSystemLibrary.Delay` 3.0)
          (`/Game/Blueprints/Widgets/InterfaceDuJoueur.NotificationMultiplicateurDeSoif` _w_interfaceutilisateur false))))
    (:`then_1`
      (if (`/Game/Blueprints/Graine.FinDuJEu` (`self.Graine_REF`))
        (`/Game/Blueprints/Parametres/PC.AfficherFinDuJEu` (`self.ControlleurDuJoueur_REF`))))))

(event `AnimMenu`
  (params (`On/Off` :type Boolean))
  (if `On/Off`
    (bind _outactor (`LevelSequencePlayer.CreateLevelSequencePlayer` "/Game/Blueprints/NewLevelSequence.NewLevelSequence"))
    (bind _output_get (set `self.AnimMenuPrincipal` _outactor))
    (`MovieSceneSequencePlayer.PlayLooping` (`LevelSequenceActor.SequencePlayer` _output_get) -1)
    (else
      (`MovieSceneSequencePlayer.Stop` (`LevelSequenceActor.SequencePlayer` (`self.AnimMenuPrincipal`))))))

(fn `UserConstructionScript`)