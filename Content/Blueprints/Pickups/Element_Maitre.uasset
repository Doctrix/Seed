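; Master pickup Blueprint for items the player can collect, with weapon-style fire and reload functions.
; Sphere overlap toggles the info widget and stencil outline, fills the widget from the Info struct, and lets Interagir call RAmasser on Personnage.
; Tirer spawns a projectile at the Muzzle socket, with a camera trace whose result is unused.
; Recharger rebuilds Info's ammo counts, and Posseder awards a one-time trophy through the game instance.
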(event `self.ReceiveBeginPlay`
  (`self.CastsRef`))

(event `FaireFeu`
  (`self.Tirer`))

(event `self.Sphere.OnComponentBeginOverlap`
  (params (OverlappedComponent :type "PrimitiveComponent Object Reference") (OtherActor :type "Actor Object Reference") (OtherComp :type "PrimitiveComponent Object Reference") (OtherBodyIndex :type Integer) (bFromSweep :type Boolean) (SweepResult :type "HitResult Structure (by ref)"))
  (bind _aspersonnage (cast `/Game/Blueprints/Personnage` OtherActor))
  (set `self.Personnage` _aspersonnage)
  (`self.Visibiliter/CustomDeph` true true)
  (set `self.PeutEtreRamasser` true)
  (`self.EnableInput` (`GameplayStatics.GetPlayerController` 0))
  (`self.AfficherInfoElement`))

(event `self.Sphere.OnComponentEndOverlap`
  (params (OverlappedComponent :type "PrimitiveComponent Object Reference") (OtherActor :type "Actor Object Reference") (OtherComp :type "PrimitiveComponent Object Reference") (OtherBodyIndex :type Integer))
  (bind _aspersonnage (cast `/Game/Blueprints/Personnage` OtherActor))
  (set `self.Personnage` _aspersonnage)
  (`self.Visibiliter/CustomDeph` false)
  (set `self.PeutEtreRamasser` false))

(event `InputAction|Interagir`
  (params (Key :type "Key Structure"))
  (:`Pressed`
    (if (`self.PeutEtreRamasser`)
      (`/Game/Blueprints/Personnage.RAmasser` (`self.Personnage`) self))))

(event `TousCacher`
  (`self.Visibiliter/CustomDeph` false)
  (`ActorComponent.K2_DestroyComponent` (`self.Sphere`)))

(event `AfficherInfoElement`
  (bind ((`Nom_29_06214B3C495C68C42BC7FFA8895D4FD2` _nom) (`Image_19_9D2608014C96C29AF3D624BDEFD5A31E` _image)) (break `/Game/Blueprints/Pickups/S_TypeItem` (`self.Info`)))
  (`self.CastsElement`)
  (`/Game/Blueprints/Widgets/w_Element.NomElement` (`self.W_Element`) _nom)
  (`/Game/Blueprints/Widgets/w_Element.ImageElement` (`self.W_Element`) _image))

(fn `Posseder`
  (params (`oui/non` :type Boolean))
  (if `oui/non`
    (`|ExecutionSequence`
      (:`then_0`
        (`/Engine/EditorBlueprintResources/StandardMacros.DoOnce` false
          (:`Completed`
            (`/Game/Blueprints/Parametres/InstanceDeJeu.AchieveTrophy` (`/Game/Blueprints/Parametres/GM.InstanceDuJeu_REF` (`self.ModeDeJeu`)) "NewEnumerator1")
            (return))))
      (:`then_1`
        _)))
  (return))

(fn `Recharger`
  (bind ((`Montant_16_BE5396AD4A7D2F06FF8D10A95D9ACAF4` _montant) (`Montantmax_17_15C0BC5244996A096AE9AAA85F98358F` _montantmax)) (break `/Game/Blueprints/Pickups/S_TypeItem` (`self.Info`)))
  (if (== _montant (`self.TailleDuChargeur`))
    _
    (elif (> _montantmax (`self.TailleDuChargeur`))
      (set `self.Info` (make `/Game/Blueprints/Pickups/S_TypeItem` :`Montant` (`self.TailleDuChargeur`) :`Montant max` (- _montantmax (`self.TailleDuChargeur`))))
      (else
        (set `self.Info` (make `/Game/Blueprints/Pickups/S_TypeItem` :`Montant` _montantmax))))))

(fn `Tirer`
  (bind _aspersonnage (cast `/Game/Blueprints/Personnage` (`GameplayStatics.GetPlayerCharacter` 0)))
  (bind _camera (`/Game/Blueprints/Personnage.Camera` _aspersonnage))
  (bind _returnvalue (`SceneComponent.K2_GetComponentLocation` _camera))
  (bind _outhit (`KismetSystemLibrary.LineTraceSingle` :`Start` _returnvalue :`End` (+ _returnvalue (* (`KismetMathLibrary.GetForwardVector` (`SceneComponent.K2_GetComponentRotation` _camera)) 1500)) :`TraceChannel` "TraceTypeQuery1" :`DrawDebugType` "ForOneFrame"))
  (`|SpawnActorFromClass` "/Game/Blueprints/Projectile.Projectile_C" (`SceneComponent.GetSocketTransform` (`self.EmplacementProjectile`) "Muzzle" "RTS_World") "Undefined" "OverrideRootScale" null null)
  (set `self.Munition` (- (`.Montant_16_BE5396AD4A7D2F06FF8D10A95D9ACAF4` (break `/Game/Blueprints/Pickups/S_TypeItem` (`self.Info`))) 1))
  (`GameplayStatics.PlaySound2D` "/Game/Audio/Water-Drops-02_Cue.Water-Drops-02_Cue" 1.0 1.0 0.0 null null))

(fn `UserConstructionScript`
  (bind (_info_nom _info_type _info_class _info_montant _info_montantmax _info_degat _info_image _info_equipernomdusocket _info_desequipernomdusocket _info_stencil) (break `/Game/Blueprints/Pickups/S_TypeItem` (`self.Info`)))
  (set `self.Info` (make `/Game/Blueprints/Pickups/S_TypeItem` _info_nom _info_type (`GameplayStatics.GetObjectClass` self) _info_montant _info_montantmax _info_degat _info_image _info_equipernomdusocket _info_desequipernomdusocket _info_stencil)))

(fn `Visibiliter/CustomDeph`
  (params (bNewVisibility :type Boolean) (bValue :type Boolean))
  (bind _sm_element (`self.SM_Element`))
  (`SceneComponent.SetVisibility` (`self.Widget`) bNewVisibility false)
  (`PrimitiveComponent.SetRenderCustomDepth` _sm_element bValue)
  (`PrimitiveComponent.SetRenderCustomDepth` (`self.SM_Element2`) bValue)
  (`PrimitiveComponent.SetCustomDepthStencilValue` _sm_element (`.Stencil_32_66E0F6FC4AA6EFBE8FE4C3A3AA06580D` (break `/Game/Blueprints/Pickups/S_TypeItem` (`self.Info`))))
  (`PrimitiveComponent.SetCustomDepthStencilValue` (`self.SM_Element2`) (`.Stencil_32_66E0F6FC4AA6EFBE8FE4C3A3AA06580D` (break `/Game/Blueprints/Pickups/S_TypeItem` (`self.Info`)))))