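; Enemy pawn that chases the player, drains 10 from their collected water on reaching them, and consumes water drops it touches.
; PawnSensing triggers AIMoveTo toward the seen Personnage, while sphere overlaps flag Eau actors as harvested or apply fixed damage from Projectiles.
; At exactly zero health it spawns an explosion emitter and destroys itself.
; On destruction it leaves the spawn point's ActivePawns list and requests a replacement enemy.
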(event `self.ReceiveBeginPlay`
  (`self.CastsRef`)
  (set `CharacterMovementComponent.MaxWalkSpeed` (`self.vitesseDeDeplacement`) (`self.CharacterMovement`)))

(event `self.PawnSensing.OnSeePawn`
  (params (Pawn :type "Pawn Object Reference"))
  (bind _aspersonnage (cast `/Game/Blueprints/Personnage` Pawn))
  (`|AIMoveTo` self (0.0 0.0 0.0) _aspersonnage 100.0
    (:`OnSuccess`
      (set `self.JoueurVu` true)
      (set `/Game/Blueprints/Personnage.QuantiteEauRecolter` (- (`/Game/Blueprints/Personnage.QuantiteEauRecolter` _aspersonnage) 10.0) _aspersonnage))
    (:`OnFail`
      (`KismetSystemLibrary.Delay` 1.0)
      (set `self.JoueurVu` false))))

(event `self.Sphere.OnComponentBeginOverlap`
  (params (OverlappedComponent :type "PrimitiveComponent Object Reference") (OtherActor :type "Actor Object Reference") (OtherComp :type "PrimitiveComponent Object Reference") (OtherBodyIndex :type Integer) (bFromSweep :type Boolean) (SweepResult :type "HitResult Structure (by ref)"))
  (`|ExecutionSequence`
    (:`then_0`
      (bind _aseau (cast `/Game/Blueprints/Eau` OtherActor))
      (bind _output_get (set `self.EauManger` true))
      (set `/Game/Blueprints/Eau.Recolter?` _output_get _aseau))
    (:`then_1`
      (cast `/Game/Blueprints/Projectile` OtherActor)
      (`self.Degats`))))

(event `Degats`
  (set `self.Santer` (- (`self.Santer`) 20.0))
  (if (== (`self.Santer`) 0.0)
    (`GameplayStatics.SpawnEmitterAttached` "/Game/Particles/FX/Eplosion.Eplosion" (`self.Mesh`) "Bone")
    (`self.K2_DestroyActor`)))

(event `self.ReceiveDestroyed`
  (bind _returnvalue (`KismetArrayLibrary.Array_RemoveItem` (`/Game/Blueprints/EmplacementDeReproductionActeur.ActivePawns` (`self.SpawnPoint_REF`)) self))
  (if _returnvalue
    (`/Game/Blueprints/EmplacementDeReproductionActeur.FaireReapparaitreUnEnnemi` (`self.SpawnPoint_REF`))))

(fn `UserConstructionScript`)