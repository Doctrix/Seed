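; CanonAO is a weapon Blueprint that fires projectiles and tracks magazine and reserve ammo.
; FaireFeu calls TirerProjectile, which spawns a Projectile at the Muzzle socket, decrements ammo without checking it and plays a sound.
; It also runs a debug camera trace whose result is unused.
; RechargerArme refills from reserve, discarding leftover rounds, while BeginPlay caches the player controller.
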(event `self.ReceiveBeginPlay`
  (`self.CastsRef`))

(event `FaireFeu`
  (`self.TirerProjectile`))

(fn `RechargerArme`
  (if (== (`self.Munition`) (`self.TailleDuChargeur`))
    _
    (elif (> (`self.MunitionMax`) (`self.TailleDuChargeur`))
      (set `self.Munition` (`self.TailleDuChargeur`))
      (set `self.MunitionMax` (- (`self.MunitionMax`) (`self.TailleDuChargeur`)))
      (else
        (set `self.Munition` (`self.MunitionMax`))
        (set `self.MunitionMax` 0)))))

(fn `TirerProjectile`
  (bind _aspersonnage (cast `/Game/Blueprints/Personnage` (`GameplayStatics.GetPlayerCharacter` 0)))
  (bind _camera (`/Game/Blueprints/Personnage.Camera` _aspersonnage))
  (bind _returnvalue (`SceneComponent.K2_GetComponentLocation` _camera))
  (bind _outhit (`KismetSystemLibrary.LineTraceSingle` :`Start` _returnvalue :`End` (+ _returnvalue (* (`KismetMathLibrary.GetForwardVector` (`SceneComponent.K2_GetComponentRotation` _camera)) 1500)) :`TraceChannel` "TraceTypeQuery1" :`DrawDebugType` "ForOneFrame"))
  (`|SpawnActorFromClass` "/Game/Blueprints/Projectile.Projectile_C" (`SceneComponent.GetSocketTransform` (`self.EmplacementProjectile`) "Muzzle" "RTS_World") "Undefined" "OverrideRootScale" null null)
  (set `self.Munition` (- (`self.Munition`) 1))
  (`GameplayStatics.PlaySound2D` "/Game/Audio/Water-Drops-02_Cue.Water-Drops-02_Cue" 1.0 1.0 0.0 null null))

(fn `UserConstructionScript`)