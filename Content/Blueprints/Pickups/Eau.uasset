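; Water pickup actor that the player (Personnage) or an enemy (Ennemi) collects by overlapping its sphere, sized in the construction script.
; A player pickup adds Quantite to their collected water and raises super water by 2, or sets it to 100 at maximum.
; Either collector decrements the GM game mode's count of water on the ground and sets Recolter, which makes Tick destroy the actor.
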(event `self.ReceiveTick`
  (params (DeltaSeconds :type "Float (single-precision)"))
  (if (`self.Recolter?`)
    (`self.K2_DestroyActor`))
  (set `self.Recolter?` false))

(event `self.Sphere.OnComponentBeginOverlap`
  (params (OverlappedComponent :type "PrimitiveComponent Object Reference") (OtherActor :type "Actor Object Reference") (OtherComp :type "PrimitiveComponent Object Reference") (OtherBodyIndex :type Integer) (bFromSweep :type Boolean) (SweepResult :type "HitResult Structure (by ref)"))
  (`|ExecutionSequence`
    (:`then_0`
      (bind _aspersonnage (cast `/Game/Blueprints/Personnage` OtherActor))
      (set `self.Recolter?` true)
      (set `self.Hero?` true)
      (`self.RecolterParLeJoueur` _aspersonnage))
    (:`then_1`
      (cast `/Game/Blueprints/IA/Ennemi` OtherActor)
      (set `self.Recolter?` true)
      (set `self.Hero?` false)))
  (bind _asgm (cast `/Game/Blueprints/Parametres/GM` (`GameplayStatics.GetGameMode`)))
  (set `/Game/Blueprints/Parametres/GM.MontantEauAuSol` (- (`/Game/Blueprints/Parametres/GM.MontantEauAuSol` _asgm) 1) _asgm))

(fn `RecolterParLeJoueur`
  (params (Personnage :type "/Game/Blueprints/Personnage Object Reference"))
  (bind _supereaurecolter (`/Game/Blueprints/Personnage.SuperEauRecolter` Personnage))
  (set `/Game/Blueprints/Personnage.QuantiteEauRecolter` (+ (`self.Quantite`) (`/Game/Blueprints/Personnage.QuantiteEauRecolter` Personnage)) Personnage)
  (if (== _supereaurecolter (`/Game/Blueprints/Personnage.SuperEauMaxRecolter` Personnage))
    (set `/Game/Blueprints/Personnage.SuperEauRecolter` 100.0 Personnage)
    (else
      (set `/Game/Blueprints/Personnage.SuperEauRecolter` (+ _supereaurecolter 2.0) Personnage))))

(fn `UserConstructionScript`
  (`SphereComponent.SetSphereRadius` (`self.Sphere`) (`self.RayonDeLaSphereCollision`) false))