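; SpawnEau is a water spawner that drops Eau or SuperEau pickups at random points inside its box, with a drip sound.
; Its SpawnGoutteEau event runs a macro that spawns according to the character's super-water state and increments the GameMode's matching ground count.
; The macro also updates the rain notification through the player controller's UI, triggers super-water management after a delay, and toggles that mode from the collected amount using hysteresis thresholds.
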(event `SpawnGoutteEau`
  (`self.SystemDeSpawn_M`))

(event `Spawn`
  (bind _box (`self.Box`))
  (bind _modedejeu (`self.ModeDeJeu`))
  (bind _returnvalue (`KismetMathLibrary.RandomPointInBoundingBox` (`SceneComponent.RelativeLocation` _box) (`BoxComponent.BoxExtent` _box)))
  (bind _output_get (`self.CastsModeDeJeu`))
  (if (`/Game/Blueprints/Personnage.SuperEauActiver?` (`/Game/Blueprints/Parametres/GM.Personnage_REF` _output_get))
    (`|SpawnActorFromClass` "/Game/Blueprints/SuperEau.SuperEau_C" (`KismetMathLibrary.Conv_VectorToTransform` _returnvalue) "Undefined" "OverrideRootScale" null null)
    (`GameplayStatics.PlaySound2D` "/Game/Audio/Water-Drops-01_Cue.Water-Drops-01_Cue" 1.0 1.0 0.0 null null)
    (set `/Game/Blueprints/Parametres/GM.MontantSuperEauAuSol` (+ (`/Game/Blueprints/Parametres/GM.MontantSuperEauAuSol` _modedejeu) 1) _modedejeu)
    (else
      (`|SpawnActorFromClass` "/Game/Blueprints/Eau.Eau_C" (`KismetMathLibrary.Conv_VectorToTransform` _returnvalue) "Undefined" "OverrideRootScale" null null)
      (`GameplayStatics.PlaySound2D` "/Game/Audio/Water-Drops-02_Cue.Water-Drops-02_Cue" 1.0 1.0 0.0 null null)
      (set `/Game/Blueprints/Parametres/GM.MontantEauAuSol` (+ (`/Game/Blueprints/Parametres/GM.MontantEauAuSol` _modedejeu) 1) _modedejeu)))
  (set `self.SpawnEau?` true))

(fn `UserConstructionScript`
  (switch `int` 0
    (:`Default`
      (`self.SpawnGoutteEau`))))