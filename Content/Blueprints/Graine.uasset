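; Seed actor the player waters to grow into a flowering plant, ending the game when its health hits zero or consumed water reaches a cap.
; A sphere overlap lets Personnage transfer collected water into the reservoir and toggles a widget and plant sprite.
; Tick drains the reservoir on delays and new days, updating health and consumed water.
; Consumed water drives a threshold macro chain that shows, scales or hides leaf, stem and flower meshes.
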(event `self.ReceiveBeginPlay`
  (`self.CastsRef`))

(event `self.ReceiveTick`
  (params (DeltaSeconds :type "Float (single-precision)"))
  (bind _gm_ref (`self.GM_REF`))
  (if (`/Game/Blueprints/GM.NouvellePartie` _gm_ref)
    (`SceneComponent.SetVisibility` (`self.ImageDeLaPlante`) true false)
    (`|ExecutionSequence`
      (:`then_0`
        (if (<= (`self.Santer`) 5.0)
          (`KismetSystemLibrary.Delay` 3.0)
          (if (> (`self.Santer`) 0.0)
            (`GameplayStatics.PlaySound2D` "/Game/Audio/water-drinking_Cue.water-drinking_Cue" 1.0 1.0 0.0 null null)
            (`KismetSystemLibrary.Delay` 1.0 :!label _label)
            (`self.ConsomationDeLeau`))
          (else
            (goto _label))))
      (:`then_1`
        (if (>= (`self.Santer`) 5.0)
          (if (`/Game/Blueprints/GM.NouvelleJourner` _gm_ref)
            (`KismetSystemLibrary.Delay` 1.0)
            (set `self.VitesseDeConsomationEau` (* (`self.MultiplicateurDeVitesse`) 1.0))
            (`self.ConsomationDeLeau`)
            (`KismetSystemLibrary.Delay` 1.0)
            (set `/Game/Blueprints/GM.NouvelleJourner` false _gm_ref)
            (`KismetSystemLibrary.PrintString` "Nouvelle journée"))))
      (:`then_2`
        (`self.Evolution`)
        (if (== (`self.Santer`) 0.0)
          (set `self.Mort?` true)
          (set `self.FinDuJEu` true :!label _label_2)
          (else
            (set `self.Mort?` false)
            (if (== (`self.EauConsommer`) 400.0)
              (goto _label_2)
              (else
                (set `self.FinDuJEu` false)))))))))

(event `ConsomationDeLeau`
  (`self.DiminutionDuReservoirEau` (`self.Reservoir`)))

(event `self.Sphere.OnComponentBeginOverlap`
  (params (OverlappedComponent :type "PrimitiveComponent Object Reference") (OtherActor :type "Actor Object Reference") (OtherComp :type "PrimitiveComponent Object Reference") (OtherBodyIndex :type Integer) (bFromSweep :type Boolean) (SweepResult :type "HitResult Structure (by ref)"))
  (bind _aspersonnage (cast `/Game/Blueprints/Personnage` OtherActor))
  (`SceneComponent.SetVisibility` (`self.Widget`) true false)
  (set `/Game/Blueprints/Personnage.PeutDonnerDeLeau` true _aspersonnage)
  (`SceneComponent.SetVisibility` (`self.ImageDeLaPlante`) false false))

(event `self.Sphere.OnComponentEndOverlap`
  (params (OverlappedComponent :type "PrimitiveComponent Object Reference") (OtherActor :type "Actor Object Reference") (OtherComp :type "PrimitiveComponent Object Reference") (OtherBodyIndex :type Integer))
  (bind _aspersonnage (cast `/Game/Blueprints/Personnage` OtherActor))
  (`SceneComponent.SetVisibility` (`self.Widget`) false false)
  (set `/Game/Blueprints/Personnage.PeutDonnerDeLeau` false _aspersonnage)
  (`SceneComponent.SetVisibility` (`self.ImageDeLaPlante`) true false))

(event `DonnerDeEau`
  (bind _reservoireaumax (`self.ReservoirEauMax`))
  (bind _personnage_ref (`/Game/Blueprints/GM.Personnage_REF` (`self.GM_REF`)))
  (bind _quantiteeaurecolter (`/Game/Blueprints/Personnage.QuantiteEauRecolter` _personnage_ref))
  (if (> _quantiteeaurecolter 0.0)
    (bind _output_get (set `self.Reservoir` (+ _quantiteeaurecolter (`self.Santer`))))
    (`GameplayStatics.PlaySound2D` "/Game/Audio/water-splash_Cue.water-splash_Cue" 1.0 1.0 1.0 null null)
    (if (> _output_get _reservoireaumax)
      (set `/Game/Blueprints/Personnage.QuantiteEauRecolter` (- _output_get _reservoireaumax) _personnage_ref)
      (else
        (set `/Game/Blueprints/Personnage.QuantiteEauRecolter` 0.0 _personnage_ref)))
    (set `self.Santer` 100.0)))

(fn `DiminutionDuReservoirEau`
  (params (Reservoir :type "Float (double-precision)"))
  (bind _vitessedeconsomationeau (`self.VitesseDeConsomationEau`))
  (bind _santer (`self.Santer`))
  (bind _eauconsommer (`self.EauConsommer`))
  (if (== Reservoir (`self.ReservoirEauMax`))
    (set `self.Reservoir` (`self.ReservoirEauMax`))
    (if (< (`self.Santer`) 80.0) :!label _label
      (set `self.Reservoir` (- Reservoir _vitessedeconsomationeau) :!label _label_2)
      (bind _output_get (set `self.EauConsommer` (+ _vitessedeconsomationeau _eauconsommer)))
      (bind _output_get_2 (set `self.Santer` (+ _output_get (`self.Santer`))))
      (if (>= _santer (`self.SanterMax`))
        (set `self.Santer` 100.0)
        (if (<= _output_get_2 0.0)
          (set `self.FinDuJEu` true)))
      (else
        (bind _output_get_3 (set `self.Santer` (- _santer 1.0) :!label _label_3))
        (if (> (`self.Reservoir`) 0.0)
          (goto _label_2)
          (elif (<= _output_get_3 50.0)
            (set `self.EauConsommer` (- _eauconsommer 1.0))))))
    (elif (== Reservoir 0.0)
      (set `self.Reservoir` 0.0)
      (goto _label_3)
      (else
        (goto _label)))))

(fn `Evolution`
  (bind _eauconsommer (`self.EauConsommer`))
  (if (>= _eauconsommer 1.0)
    (`SceneComponent.SetVisibility` (`self.Graine_SM`) false false)
    (`SceneComponent.SetVisibility` (`self.Tige_SM`) true false)
    (`self.FaireEvoluer` _eauconsommer)
    (return)))

(fn `UserConstructionScript`
  (`SphereComponent.SetSphereRadius` (`self.Sphere`) (`self.SphereRadius`) true)
  (`BillboardComponent.SetSprite` (`self.ImageDeLaPlante`) (`self.ImageActuelDeLaPlante`)))