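; Eau is a water pickup actor that refills the player's water when a Personnage overlaps its collision Sphere.
; On overlap it adds its Eau amount to the character's Reservoir, then destroys itself.
; It also increments SuperWater by a fixed step, or sets it to a hardcoded value when it exactly equals SuperWaterMax.
; The construction script sizes the Sphere from RayonDeLaSphereCollision.
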(event `self.Sphere.OnComponentBeginOverlap`
  (params (OverlappedComponent :type "PrimitiveComponent Object Reference") (OtherActor :type "Actor Object Reference") (OtherComp :type "PrimitiveComponent Object Reference") (OtherBodyIndex :type Integer) (bFromSweep :type Boolean) (SweepResult :type "HitResult Structure (by ref)"))
  (bind _aspersonnage (cast `/Game/Blueprints/Personnage` OtherActor))
  (set `/Game/Blueprints/Personnage.Reservoir` (+ (`/Game/Blueprints/Personnage.Reservoir` _aspersonnage) (`self.eau`)) _aspersonnage)
  (bind _superwater (`/Game/Blueprints/Personnage.SuperWater` _aspersonnage))
  (if (== _superwater (`/Game/Blueprints/Personnage.SuperWater_Max` _aspersonnage))
    (set `/Game/Blueprints/Personnage.SuperWater` 100.0 _aspersonnage)
    (else
      (set `/Game/Blueprints/Personnage.SuperWater` (+ _superwater 2.0) _aspersonnage)))
  (`self.K2_DestroyActor`))

(fn `UserConstructionScript`
  (`SphereComponent.SetSphereRadius` (`self.Sphere`) (`self.RayonDeLaSphereCollision`) false))